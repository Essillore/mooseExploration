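; BP_ScalingWalls is a wall Blueprint that animates the texture scale of a moving patterned material.
; On BeginPlay, TimelineScale drives the TexScaleXYPosXY vector parameter on SMWall2's materials.
; Each time the timeline finishes, it waits briefly and reverses from the end, so the reverse pass repeats.
; Dynamic material instances are created in BeginPlay and the construction script, but neither is visibly assigned to a mesh.
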(event `self.ReceiveBeginPlay`
  (`KismetMaterialLibrary.CreateDynamicMaterialInstance` "/Game/VL_PsyPatterns/Materials/M_MasterMaterial_Moving.M_MasterMaterial_Moving")
  (bind (_direction _settingscale) (`Timeline|TimelineScale` :`NewTime` (`KismetSystemLibrary.GetGameTimeInSeconds`) :!label _label)
    (:`Update`
      (`MeshComponent.SetVectorParameterValueOnMaterials` (`self.SM_Wall_2`) (`self.Tex_ScaleXY_PosXY`) (`KismetMathLibrary.Conv_DoubleToVector` _settingscale)))
    (:`Finished`
      (`KismetSystemLibrary.Delay` 0.2)
      (goto _label :!via `ReverseFromEnd`))))

(fn `UserConstructionScript`
  (bind _scalar (`self.Scalar`))
  (bind _returnvalue (`KismetMaterialLibrary.CreateDynamicMaterialInstance` "/Game/VL_PsyPatterns/Materials/MI_Material_Type12.MI_Material_Type12"))
  (`MaterialInstanceDynamic.SetScalarParameterValue` _returnvalue _scalar 0.0)
  (set `self.TimelineScale` (`self.TimelineScale`))
  (set `self.Scalar` _scalar))