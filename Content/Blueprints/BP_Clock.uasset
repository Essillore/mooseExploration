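; BP_Clock is a clock that keeps a running SecondOfDay counter and converts it to hours, minutes and seconds.
; Tick waits on a Delay of frame time multiplied by ClockSpeed, so larger values tick slower, then TickingTo86400 adds one second with no wrap at 86400.
; SecondsToTime splits the count by whole-and-remainder division, but Tick discards the result and GetTime returns none of it.
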(event `self.ReceiveTick`
  (params (DeltaSeconds :type "Float (single-precision)"))
  (`KismetSystemLibrary.Delay` (* DeltaSeconds (`self.ClockSpeed`)))
  (bind _secondsofday (`self.TickingTo86400`))
  (`self.SecondsToTime` _secondsofday))

(fn `GetTime`
  (params (Hours :type Integer) (Minutes :type Integer) (Seconds :type Integer))
  (`self.SecondsToTime` (`self.SecondOfDay`))
  (return))

(fn `SecondsToTime`
  (params (SecondsOfDay :type "Float (double-precision)"))
  (returns (Hours :type Integer) (Minutes :type Integer) (Seconds :type Integer))
  (bind (_remainder _returnvalue) (`KismetMathLibrary.FMod` SecondsOfDay 60.0))
  (bind _output_get (set `self.Minutes` _returnvalue))
  (bind (_remainder_2 _returnvalue_2) (`KismetMathLibrary.FMod` (`KismetMathLibrary.Conv_IntToDouble` _output_get) 60.0))
  (bind _output_get_2 (set `self.Hours` _returnvalue_2))
  (bind _output_get_3 (set `self.Seconds` (`KismetMathLibrary.FTrunc` _remainder)))
  (return _output_get_2 (`KismetMathLibrary.FTrunc` _remainder_2) _output_get_3))

(fn `TickingTo86400`
  (returns (SecondsOfDay :type "Float (double-precision)"))
  (bind _output_get (set `self.SecondOfDay` (+ (`self.SecondOfDay`) 1.0)))
  (return _output_get))

(fn `UserConstructionScript`)